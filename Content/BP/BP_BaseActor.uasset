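; BP_BaseActor is an autonomous agent on the XZ plane that investigates nearby BP_BasePlace actors and collects facts from them.
; When idle, the looping ASeM timer uses a box trace to pick the nearest unvisited place, then starts a timer-driven move or investigation.
; Investigation prints the character's reaction and infers DemonSummoned once Book and Circle are known.
; Curve-scored utility selection between Eat and Work exists but is disconnected.
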(event EventBeginPlay
  (bind _returnvalue (Utilities|Time|SetTimerbyFunctionName 0 "ASeM" 1.0 true))
  (Variables|Default|SetTH_ASeM _returnvalue))

(event EventTick
  (params (DeltaSeconds :type Float%20%28single-precision%29))
  (Utilities|FlowControl|Sequence
    (:then_0
      (Rendering|Debug|DrawDebugBox (Transformation|GetActorLocation) "5.000000, 0,5.000000" "(R=1.000000,G=0.000000,B=0.017203,A=1.000000)" "0, 0, 0" 0.0 0.0))))

(fn ConstructionScript)

(fn ActionMoveTo(Actor)
  (params (TargetActor :type Actor%20Object%20Reference))
  (Development|PrintString "Action:MoveTo")
  (Variables|Default|SetisHaveTask true)
  (bind _returnvalue (Utilities|Time|SetTimerbyEvent (EventDispatchers|CreateEvent :!event ActionSMove) (Utilities|Time|GetWorldDeltaSeconds) true))
  (Variables|Default|SetTH_Action _returnvalue))

(fn ASeM
  (if (not (Variables|Default|GetisHaveTask))
    (bind _output_get (Variables|Default|SetTargerActor (CallFunction|SensorVision)))
    (Utilities|IsValid _output_get
      (:Is%20Valid
        (if (< (CallFunction|CheckDistance(ToActor) (Variables|Default|GetTargerActor)) 2.0)
          (CallFunction|ActionSInvestigate)
          (else
            (CallFunction|ActionMoveTo(Actor)))))
      (:Is%20Not%20Valid
        (Development|PrintString "Invalid Target!" true true "(R=1.000000,G=0.000000,B=0.005046,A=1.000000)")))))

(fn ActionSMove
  (bind _returnvalue (Transformation|GetActorLocation))
  (bind _returnvalue_2 (Transformation|GetActorLocation))
  (bind _targeractor (Variables|Default|GetTargerActor))
  (bind _targeractor_2 (Variables|Default|GetTargerActor))
  (bind (_x _y _z) (Math|Vector|BreakVector _returnvalue))
  (bind _returnvalue_3 (Transformation|GetActorLocation _targeractor_2))
  (bind (_x_2 _y_2 _z_2) (Math|Vector|BreakVector _returnvalue_2))
  (bind _returnvalue_4 (Transformation|GetActorLocation _targeractor))
  (bind (_x_3 _y_3 _z_3) (Math|Vector|BreakVector _returnvalue_3))
  (bind (_x_4 _y_4 _z_4) (Math|Vector|BreakVector _returnvalue_4))
  (Utilities|IsValid (Variables|Default|GetTargerActor)
    (:Is%20Valid
      (if (< (Math|Vector|VectorLength (- (Math|Vector|MakeVector _x_4 0.0 _z_4) (Math|Vector|MakeVector _x_2 0.0 _z_2))) 2.0)
        (CallFunction|ClearAction)
        (Development|PrintString "Reached!" true true "(R=0.121010,G=1.000000,B=0.000000,A=1.000000)")
        (else
          (Transformation|SetActorLocation (+ (Transformation|GetActorLocation) (* (Math|Vector|Normalize (- (Math|Vector|MakeVector _x_3 0.0 _z_3) (Math|Vector|MakeVector _x 0.0 _z))) (* (Variables|Default|GetMovement_Speed) (Utilities|Time|GetWorldDeltaSeconds)))) false false))))
    (:Is%20Not%20Valid
      (CallFunction|ClearAction)
      (Development|PrintString "Invalid Target!" true true "(R=1.000000,G=0.000000,B=0.017203,A=1.000000)"))))

(fn ClearAction
  (Utilities|Time|ClearandInvalidateTimerbyHandle (Variables|Default|GetTH_Action))
  (Variables|Default|SetisHaveTask false))

(fn ActionEat
  (Variables|Default|SetTargerActor (Variables|Default|GetEatPlace))
  (if (< (CallFunction|CheckDistance(ToActor)) 2.0)
    (CallFunction|ActionSEat)
    (else
      (CallFunction|ActionMoveTo(Actor)))))

(fn ActionWork
  (Variables|Default|SetTargerActor (Variables|Default|GetWorkPlace))
  (if (< (CallFunction|CheckDistance(ToActor)) 2.0)
    (CallFunction|ActionSWork)
    (else
      (CallFunction|ActionMoveTo(Actor)))))

(fn CheckDistance(ToActor)
  (params (TargetActor :type Actor%20Object%20Reference))
  (bind _returnvalue (Transformation|GetActorLocation TargetActor))
  (bind _returnvalue_2 (Transformation|GetActorLocation))
  (bind (_x _y _z) (Math|Vector|BreakVector _returnvalue))
  (bind (_x_2 _y_2 _z_2) (Math|Vector|BreakVector _returnvalue_2))
  (return (Math|Vector|VectorLength (- (Math|Vector|MakeVector _x 0.0 _z) (Math|Vector|MakeVector _x_2 0.0 _z_2)))))

(fn ActionSEat
  (Development|PrintString "Action:S_Eat")
  (Variables|Default|SetisHaveTask true)
  (bind _returnvalue (Utilities|Time|SetTimerbyEvent (EventDispatchers|CreateEvent :!event ActionFinishEat) 1.0))
  (Variables|Default|SetTH_Action _returnvalue))

(fn ActionFinishEat
  (CallFunction|ClearAction)
  (Development|PrintString "Eated!" true true "(R=0.121010,G=1.000000,B=0.000000,A=1.000000)")
  (Variables|Default|SetHunger (Math|Float|Max(Float) (- (Variables|Default|GetHunger) 7e+01) 0.0)))

(fn AEM
  (return (.Value (Utilities|Map|Find (Utilities|Map|MakeMap (Scorer|ScorerHunger) (Utilities|Name|MakeLiteralName "Eat") (Scorer|ScorerWork) (Utilities|Name|MakeLiteralName "Work")) (Math|Float|Max(Float) (Scorer|ScorerHunger) (Scorer|ScorerWork))))))

(fn UpdateNeeds
  (Variables|Default|SetHunger (select (< (Variables|Default|GetHunger) 1e+02) (+ (Variables|Default|GetHunger) 0.6) (Variables|Default|GetHunger))))

(fn ScorerHunger
  (return (Math|Curves|GetFloatValue (Variables|Default|GetCurve_Hunger) (Variables|Default|GetHunger))))

(fn ScorerWork
  (return 0.5))

(fn ActionSWork
  (Development|PrintString "Action:S_Work")
  (Variables|Default|SetisHaveTask true)
  (bind _returnvalue (Utilities|Time|SetTimerbyEvent (EventDispatchers|CreateEvent :!event ActionFinishWork) 3.0))
  (Variables|Default|SetTH_Action _returnvalue))

(fn ActionFinishWork
  (CallFunction|ClearAction)
  (Development|PrintString "Worked!" true true "(R=0.121010,G=1.000000,B=0.000000,A=1.000000)"))

(fn SensorVision
  (bind _returnvalue (Transformation|GetActorLocation))
  (bind _outhits (Class|KismetSystemLibrary|BoxTraceMulti _returnvalue _returnvalue "300.000000,100.000000,300.000000" "0, 0, 0" "TraceTypeQuery1" false 0 "None" true "(R=1.000000,G=0.000000,B=0.000000,A=1.000000)" "(R=0.000000,G=1.000000,B=0.000000,A=1.000000)" 1.0))
  (for _array_element _outhits
    (bind _asbp_base_place (Utilities|Casting|CastToBP_BasePlace (.HitActor (Collision|BreakHitResult _array_element))))
    (if (not (Variables|/Game/BP/BP_BasePlace.BP_BasePlace_C|GetisInvestigated _asbp_base_place))
      (Utilities|Array|Add (LocalVariables|GetUnvisitedPlaces) _asbp_base_place)))
  (LocalVariables|SetMinDistance 1e+07)
  (for _array_element_2 (LocalVariables|GetUnvisitedPlaces)
    (if (< (CallFunction|CheckDistance(ToActor) _array_element_2) (LocalVariables|GetMinDistance))
      (LocalVariables|SetMinDistance (CallFunction|CheckDistance(ToActor) _array_element_2))
      (LocalVariables|SetResultPlace _array_element_2)))
  (return (LocalVariables|GetResultPlace)))

(fn ActionSInvestigate
  (Development|PrintString "Action:S_Investigate")
  (Variables|Default|SetisHaveTask true)
  (bind _returnvalue (Utilities|Time|SetTimerbyEvent (EventDispatchers|CreateEvent :!event ActionFinishInvestigate) 3.0))
  (Variables|Default|SetTH_Action _returnvalue))

(fn ActionFinishInvestigate
  (bind _struct_fact (Utilities|Struct|MakeStruct_Fact "DemonSummoned" "Культ призвал Демона!"))
  (bind (_id _characterreaction) (Utilities|Struct|BreakStruct_Fact _struct_fact))
  (CallFunction|ClearAction)
  (Development|PrintString "Investigated!" true true "(R=0.121010,G=1.000000,B=0.000000,A=1.000000)")
  (bind _fact (Default|Investigated (.AsBP%20Base%20Place (Utilities|Casting|CastToBP_BasePlace (Variables|Default|GetTargerActor)))))
  (Utilities|Array|Add (Variables|Default|GetFacts_Known) (.ID (Utilities|Struct|BreakStruct_Fact _fact)))
  (Development|PrintText (.CharacterReaction (Utilities|Struct|BreakStruct_Fact _fact)) true true "(R=1.000000,G=0.000000,B=0.866851,A=1.000000)")
  (if (and (> (Utilities|Array|FindItem (Variables|Default|GetFacts_Known) "Book") -1) (> (Utilities|Array|FindItem (Variables|Default|GetFacts_Known) "Circle") -1))
    (Utilities|Array|Add (Variables|Default|GetFacts_Known) _id)
    (Development|PrintText _characterreaction true true "(R=1.000000,G=0.000000,B=0.866851,A=1.000000)")))